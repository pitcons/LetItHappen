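; First-person player character that places Human and Polizei actors with left and right clicks in an interactive scene.
; A camera line trace each Tick sets the spawn point, swaps cursor meshes and flags hovered columns, speakers or the LetItHappen target.
; Left-click on these teleports the player, randomly stops or plays music, or, given enough Humans, plays speeches and sets people, avtozaks and fences simulating physics, mostly without gravity.
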(event `InputAxis|WalkFB`
  (params (AxisValue :type "Float (single-precision)"))
  (`self.AddMovementInput` (`self.GetActorForwardVector`) AxisValue))

(event `InputAxis|LookUD`
  (params (AxisValue :type "Float (single-precision)"))
  (`self.AddControllerPitchInput` (/ AxisValue 2.0)))

(event `self.ReceiveBeginPlay`)

(event `InputAxis|WalkLR`
  (params (AxisValue :type "Float (single-precision)"))
  (`self.AddMovementInput` (`self.GetActorRightVector`) AxisValue))

(event `InputAxis|LookRL`
  (params (AxisValue :type "Float (single-precision)"))
  (`self.AddControllerYawInput` (/ AxisValue 2.0)))

(event `Key|LeftShift`
  (params (Key :type "Key Structure" :default "AnyKey"))
  (bind _charactermovement (`self.CharacterMovement`))
  (:`Pressed`
    (set `CharacterMovementComponent.MaxWalkSpeed` 1200.0 _charactermovement))
  (:`Released`
    (set `CharacterMovementComponent.MaxWalkSpeed` 700.0 _charactermovement)))

(event `Key|SpaceBar`
  (params (Key :type "Key Structure" :default "AnyKey"))
  (:`Pressed`
    (`self.Jump`)))

(event `Key|F12`
  (params (Key :type "Key Structure" :default "AnyKey"))
  (:`Pressed`
    (`KismetSystemLibrary.ExecuteConsoleCommand` "HighResShot  1")))

(event `self.ReceiveTick`
  (params (DeltaSeconds :type "Float (single-precision)"))
  (bind _cursorhand (`self.cursorHand`))
  (bind _cursor (`self.cursor`))
  (bind _cursorhand_2 (`self.cursorHand`))
  (bind _cursorarrow (`self.cursorArrow`))
  (bind _hitresult (`self.LineTracing`))
  (bind (_bblockinghit _binitialoverlap _time _location _impactpoint _normal _impactnormal _physmat _hitactor) (`GameplayStatics.BreakHitResult` _hitresult))
  (set `self.humanSpawnLocation` _location)
  (bind _returnvalue (`GameplayStatics.GetObjectClass` _hitactor))
  (if (== _returnvalue "/Game/Blueprints/aColumn_B.aColumn_B_C")
    (`SceneComponent.SetVisibility` (`self.cursorArrow`) true false)
    (`SceneComponent.SetVisibility` (`self.cursor`) false false)
    (`SceneComponent.SetVisibility` (`self.cursorHand`) false false)
    (`MeshComponent.SetVectorParameterValueOnMaterials` _cursorarrow "color1" (`KismetMathLibrary.MakeVector` 0.0 0.065 0.135))
    (`MeshComponent.SetVectorParameterValueOnMaterials` _cursorarrow "color2" (`KismetMathLibrary.MakeVector` 0.211 0.396 0.475))
    (set `self.isItColumn` true)
    (set `self.isItTxt` false)
    (set `self.isItSpeaker` false)
    (else
      (bind _outactors (`GameplayStatics.GetAllActorsOfClass` "/Game/Blueprints/human.human_C"))
      (if (and (== _returnvalue "/Game/Blueprints/letItHappen.letItHappen_C") (>= (`KismetArrayLibrary.Array_Length` _outactors) 20))
        (`KismetSystemLibrary.PrintString` "Hello" false false)
        (`SceneComponent.SetVisibility` _cursorhand true false)
        (`/Game/Blueprints/Utils.CreateDynamicMat` _cursorhand (struct) (struct) 0 "/Game/Materials/cursorOneColor.cursorOneColor" false 1.0 1.0)
        (`/Game/Blueprints/Utils.CreateDynamicMat` _cursorhand (struct :`R` 1.0 :`G` 1.0 :`B` 1.0 :`A` 1.0) (struct) 1 "/Game/Materials/cursorOneColor.cursorOneColor" false 1.0 1.0)
        (`SceneComponent.SetVisibility` (`self.cursorArrow`) false false)
        (`SceneComponent.SetVisibility` (`self.cursor`) false false)
        (set `self.isItTxt` true)
        (set `self.isItSpeaker` false)
        (set `self.isItColumn` false)
        (elif (== _returnvalue "/Game/Blueprints/speaker.speaker_C")
          (`SceneComponent.SetVisibility` _cursorhand_2 true false)
          (`/Game/Blueprints/Utils.CreateDynamicMat` _cursorhand_2 (struct :`G` 0.52549 :`B` 0.462745 :`A` 1.0) (struct) 0 "/Game/Materials/cursorOneColor.cursorOneColor" false 1.0 1.0)
          (`/Game/Blueprints/Utils.CreateDynamicMat` _cursorhand_2 (struct :`R` 0.52549 :`G` 0.015087 :`A` 1.0) (struct) 1 "/Game/Materials/cursorOneColor.cursorOneColor" false 1.0 1.0)
          (`SceneComponent.SetVisibility` (`self.cursorArrow`) false false)
          (`SceneComponent.SetVisibility` (`self.cursor`) false false)
          (set `self.isItSpeaker` true)
          (set `self.isItColumn` false)
          (set `self.isItTxt` false)
          (else
            (`SceneComponent.SetVisibility` (`self.cursorArrow`) false false)
            (`SceneComponent.SetVisibility` (`self.cursorHand`) false false)
            (set `self.isItColumn` false)
            (set `self.isItTxt` false)
            (set `self.isItSpeaker` false)
            (if _bblockinghit
              (`SceneComponent.SetVisibility` _cursor true false)
              (else
                (`SceneComponent.SetVisibility` _cursor false false)))))))))

(event `Key|Three`
  (params (Key :type "Key Structure" :default "AnyKey")))

(event `Key|Four`
  (params (Key :type "Key Structure" :default "AnyKey")))

(event `Key|LeftMouseButton`
  (params (Key :type "Key Structure" :default "AnyKey"))
  (bind _cursor (`self.cursor`))
  (bind _music (`/Game/Blueprints/speaker.music` (`self.speaker1`)))
  (:`Pressed`
    (`MeshComponent.SetVectorParameterValueOnMaterials` _cursor "color1" (`KismetMathLibrary.MakeVector` 0.0 0.065 0.135))
    (`MeshComponent.SetVectorParameterValueOnMaterials` _cursor "color2" (`KismetMathLibrary.MakeVector` 0.5 0.4 0.3))
    (if (`self.isItColumn`)
      (`self.K2_SetActorLocation` self (-1455.0 -2415.0 1949.0) false false)
      (elif (`self.isItSpeaker`)
        ;[1 1 1] music on/off
        (if (== (`KismetMathLibrary.RandomIntegerInRange` 0 3) 0)
          (`AudioComponent.Stop` _music)
          (else
            (`AudioComponent.Play` _music 0.0)))
        (else
          (bind _outactors (`GameplayStatics.GetAllActorsOfClass` "/Game/Blueprints/human.human_C"))
          (bind _returnvalue (>= (`KismetArrayLibrary.Array_Length` _outactors) 20))
          (if (and (`self.isItTxt`) _returnvalue)
            (`self.HumanPhysicsOn`)
            (`self.HumanPhysicsOn`)
            (`self.HumanPhysicsOn`)
            (`self.AvtozakPhysicsOn`)
            (`self.AvtozakPhysicsOn`)
            (`self.AvtozakPhysicsOn`)
            (`self.fenceCelebrPhysicsOn`)
            (for _array_element _outactors
              (`AudioComponent.Play` (`/Game/Blueprints/human.speech` _array_element) 0.0))
            (`/Engine/EditorBlueprintResources/StandardMacros.DoOnce` false
              (:`Completed`
                (set `self.isFirstTimeItHappen` true)))
            (else
              (if _returnvalue
                (set `self.isUsMany` true))
              (if (!= (`self.isFirstTime3or4pressed`) true)
                (`|SpawnActorFromClass` "/Game/Blueprints/human.human_C" (`KismetMathLibrary.MakeTransform` (`self.humanSpawnLocation`) (`KismetMathLibrary.MakeRotator` 0.0 0.0 (`KismetMathLibrary.RandomFloatInRange` 0.0 180.0)) (1.0 1.0 1.0)) "Undefined" "OverrideRootScale")
                (if (`self.isFirstTimeItHappen`)
                  (`self.HumanPhysicsOn`)
                  (`self.HumanPhysicsOn`)
                  (`self.HumanPhysicsOn`))))))))))

(event `Key|RightMouseButton`
  (params (Key :type "Key Structure" :default "AnyKey"))
  (bind _cursor (`self.cursor`))
  (:`Pressed`
    (`MeshComponent.SetVectorParameterValueOnMaterials` _cursor "color1" (`KismetMathLibrary.MakeVector` 0.0 0.0 0.0))
    (`MeshComponent.SetVectorParameterValueOnMaterials` _cursor "color2" (`KismetMathLibrary.MakeVector` 0.1 0.1 0.1))
    (`|SpawnActorFromClass` "/Game/Blueprints/polizei.polizei_C" (`KismetMathLibrary.MakeTransform` (`self.humanSpawnLocation`) (`KismetMathLibrary.MakeRotator` 0.0 0.0 (`KismetMathLibrary.RandomFloatInRange` 0.0 180.0)) (1.0 1.0 1.0)) "Undefined" "OverrideRootScale")
    (if (`self.isFirstTimeItHappen`)
      (`self.HumanPhysicsOn`)
      (`self.HumanPhysicsOn`)
      (`self.HumanPhysicsOn`))))

(fn `AvtozakPhysicsOn`
  (bind _outactors (`GameplayStatics.GetAllActorsOfClass` "/Game/Blueprints/avtozak.avtozak_C"))
  (for _array_element _outactors
    (for _array_element_2 (`SceneComponent.GetChildrenComponents` (`/Game/Blueprints/avtozak.DefaultSceneRoot` _array_element) true)
      (bind _asstatic_mesh_component (cast `StaticMeshComponent` _array_element_2))
      (`PrimitiveComponent.SetSimulatePhysics` _asstatic_mesh_component true)
      (`PrimitiveComponent.SetEnableGravity` _asstatic_mesh_component false))))

(fn `fenceCelebrPhysicsOn`
  (bind _outactors (`GameplayStatics.GetAllActorsOfClass` "/Game/Blueprints/fenceCelebration.fenceCelebration_C"))
  (for _array_element _outactors
    (`PrimitiveComponent.SetSimulatePhysics` (`/Game/Blueprints/fenceCelebration.fenceCelebration` _array_element) true)))

(fn `FramesPhysicsOn`)

(fn `HumanPhysicsOn`
  (bind _outactors (`GameplayStatics.GetAllActorsOfClass` "/Game/Blueprints/human.human_C"))
  (for _array_element _outactors
    (for _array_element_2 (`SceneComponent.GetChildrenComponents` (`/Game/Blueprints/human.DefaultSceneRoot` _array_element) true)
      (bind _asstatic_mesh_component (cast `StaticMeshComponent` _array_element_2))
      (`PrimitiveComponent.SetSimulatePhysics` _asstatic_mesh_component true)
      (`PrimitiveComponent.SetAngularDamping` _asstatic_mesh_component 0.0)
      (`PrimitiveComponent.SetEnableGravity` _asstatic_mesh_component false)))
  (bind _outactors_2 (`GameplayStatics.GetAllActorsOfClass` "/Game/Blueprints/polizei.polizei_C"))
  (for _array_element_3 _outactors_2
    (for _array_element_4 (`SceneComponent.GetChildrenComponents` (`/Game/Blueprints/polizei.Cube` _array_element_3) true)
      (bind _asstatic_mesh_component_2 (cast `StaticMeshComponent` _array_element_4))
      (`KismetSystemLibrary.PrintString` (`KismetSystemLibrary.GetDisplayName` _asstatic_mesh_component_2) false false)
      (`PrimitiveComponent.SetSimulatePhysics` _asstatic_mesh_component_2 true)
      (`PrimitiveComponent.SetAngularDamping` _asstatic_mesh_component_2 0.0)
      (`PrimitiveComponent.SetEnableGravity` _asstatic_mesh_component_2 false))))

(fn `LineTracing`
  (returns (hitResult :type "HitResult Structure"))
  (bind _camera (`self.Camera`))
  (bind _returnvalue (`SceneComponent.K2_GetComponentLocation` _camera))
  (bind _outhit (`KismetSystemLibrary.LineTraceSingleForObjects` _returnvalue (+ _returnvalue (* (`KismetMathLibrary.GetForwardVector` (`SceneComponent.K2_GetComponentRotation` _camera)) 100000.0)) (`self.objectsForTracing`)))
  (return _outhit))

(fn `UserConstructionScript`
  (bind _cursor (`self.cursor`))
  (`MeshComponent.SetVectorParameterValueOnMaterials` _cursor "color1" (`KismetMathLibrary.MakeVector` 0.0 0.065 0.135))
  (`MeshComponent.SetVectorParameterValueOnMaterials` _cursor "color2" (`KismetMathLibrary.MakeVector` 0.5 0.4 0.3)))
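; Utility functions that create dynamic material instances on mesh components and set their look through named parameters.
; CreateDynamicMatTextures sets UV tiling and optionally picks a random texture from a supplied array.
; CreateDynamicMat applies two colors and optional UV tiling, then returns the instance.
; GenerateColor calls CreateDynamicMat with a horizontal two-color gradient material, then overrides both colors with random dark tints.
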(fn `CreateDynamicMat`
  (params (meshComponent :type "PrimitiveComponent Object Reference") (color1 :type "LinearColor Structure") (color2 :type "LinearColor Structure") (elementIndex :type Integer) (sourceMaterial :type "Material Object Reference") (setUVs :type Boolean) (U :type "Float (double-precision)") (V :type "Float (double-precision)"))
  (returns (dynamicMaterial :type "MaterialInstanceDynamic Object Reference"))
  (locals (dynamicMat :type "MaterialInstanceDynamic Object Reference"))
  (bind _returnvalue (`PrimitiveComponent.CreateDynamicMaterialInstance` meshComponent elementIndex sourceMaterial))
  (bind _output_get (set `local.dynamicMat` _returnvalue))
  (`MaterialInstanceDynamic.SetVectorParameterValue` _output_get "color1" color1)
  (`MaterialInstanceDynamic.SetVectorParameterValue` _output_get "color2" color2)
  (if (== setUVs true)
    (`MaterialInstanceDynamic.SetScalarParameterValue` _output_get "U" U)
    (`MaterialInstanceDynamic.SetScalarParameterValue` _output_get "V" V))
  (return _output_get))

(fn `CreateDynamicMatTextures`
  (params (meshComponent :type "PrimitiveComponent Object Reference") (sourceMaterial :type "Material Object Reference") (textures :type "Array of Texture2D Object Reference") (randomizeTextures :type Boolean) (tilesU :type "Float (double-precision)") (tilesV :type "Float (double-precision)") (elementIndex :type Integer))
  (locals (dynamicMat :type "MaterialInstanceDynamic Object Reference"))
  (bind _returnvalue (`PrimitiveComponent.CreateDynamicMaterialInstance` meshComponent elementIndex sourceMaterial))
  (bind _output_get (set `local.dynamicMat` _returnvalue))
  (`MaterialInstanceDynamic.SetScalarParameterValue` _output_get "U" tilesU)
  (`MaterialInstanceDynamic.SetScalarParameterValue` _output_get "V" tilesV)
  (if randomizeTextures
    (`MaterialInstanceDynamic.SetTextureParameterValue` _output_get "texture" (`KismetArrayLibrary.Array_Get` textures (`KismetMathLibrary.RandomIntegerInRange` 0 (`KismetArrayLibrary.Array_Length` textures))))))

(fn `GenerateColor`
  (bind _linearcolor (make `LinearColor` (`KismetMathLibrary.RandomFloatInRange` 0.05 0.09) (`KismetMathLibrary.RandomFloatInRange` 0.04 0.09) (`KismetMathLibrary.RandomFloatInRange` 0.01 0.09) 1.0))
  (bind _dynamicmaterial (`self.CreateDynamicMat` null (struct) (struct) 1 "/Game/Materials/simple2colorGradHorizontal.simple2colorGradHorizontal"))
  (`MaterialInstanceDynamic.SetVectorParameterValue` _dynamicmaterial "color1" _linearcolor)
  (`MaterialInstanceDynamic.SetVectorParameterValue` _dynamicmaterial "color2" _linearcolor))
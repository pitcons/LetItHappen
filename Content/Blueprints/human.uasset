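; Procedurally randomized human actor built from body-part meshes, with a shovel at the right hand.
; The construction script randomizes proportions, then positions limbs, shovel and physics constraints from component bounds.
; It randomizes face, hair, skin and clothing colors through dynamic materials, using two-color gradient split points for sleeve, pants and coat lengths.
; Tick accumulates time to blink at random intervals by squashing the eyes' Z scale and restoring it.
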(event `self.ReceiveTick`
  (params (DeltaSeconds :type "Float (single-precision)"))
  (bind _returnvalue (`KismetMathLibrary.RandomFloatInRange` 3.0 10.0))
  (bind _output_get (set `self.tickDelay` (+ DeltaSeconds (`self.tickDelay`))))
  (set `self.eyesTime` _returnvalue)
  (if (> _output_get _returnvalue)
    (`self.EyesBlink`)
    (if (>= _output_get (+ (`self.eyesTime`) 0.001))
      (`SceneComponent.SetRelativeScale3D` (`self.eye1`) (`self.eyesScale`))
      (`SceneComponent.SetRelativeScale3D` (`self.eye2`) (`self.eyesScale`))
      (set `self.tickDelay` 0.0))))

(fn `EyesBlink`
  (bind _eye1 (`self.eye1`))
  (bind _returnvalue (`KismetMathLibrary.MakeVector` (.x (`SceneComponent.RelativeScale3D` _eye1)) (.y (`SceneComponent.RelativeScale3D` _eye1)) 0.002))
  (`SceneComponent.SetRelativeScale3D` _eye1 _returnvalue)
  (`SceneComponent.SetRelativeScale3D` (`self.eye2`) _returnvalue))

(fn `GenerateColors`
  (set `self.eyesColor` (make `LinearColor` (`KismetMathLibrary.RandomFloatInRange` 0.0 0.2) (`KismetMathLibrary.RandomFloatInRange` 0.0 0.2) (`KismetMathLibrary.RandomFloatInRange` 0.0 0.2) 1.0))
  (set `self.coatColor` (make `LinearColor` (`KismetMathLibrary.RandomFloatInRange` 0.0 0.7) (`KismetMathLibrary.RandomFloatInRange` 0.0 0.7) (`KismetMathLibrary.RandomFloatInRange` 0.0 0.7) 1.0))
  (set `self.pantsColor` (make `LinearColor` (`KismetMathLibrary.RandomFloatInRange` 0.0 0.7) (`KismetMathLibrary.RandomFloatInRange` 0.0 0.7) (`KismetMathLibrary.RandomFloatInRange` 0.0 0.7) 1.0))
  (set `self.shoesColor` (make `LinearColor` (`KismetMathLibrary.RandomFloatInRange` 0.0 0.1) (`KismetMathLibrary.RandomFloatInRange` 0.0 0.1) (`KismetMathLibrary.RandomFloatInRange` 0.0 0.1) 1.0)))

(fn `UserConstructionScript`
  (bind _returnvalue (`KismetMathLibrary.RandomFloatInRange` 1.0 2.0))
  (bind _body (`self.body`))
  (bind _hand1 (`self.hand1`))
  (bind _eye1 (`self.eye1`))
  (bind _eye2 (`self.eye2`))
  (bind _eyescolor (`self.eyesColor`))
  (bind _mouth (`self.mouth`))
  (bind _shovel (`self.shovel`))
  (bind (_origin _boxextent) (`KismetSystemLibrary.GetComponentBounds` _hand1))
  (bind (_origin_2 _boxextent_2) (`KismetSystemLibrary.GetComponentBounds` _body))
  (bind _linearcolor (make `LinearColor` (`KismetMathLibrary.RandomFloatInRange` 0.1 0.18) (`KismetMathLibrary.RandomFloatInRange` 0.02 0.09) (`KismetMathLibrary.RandomFloatInRange` 0.01 0.09) 1.0))
  (bind _linearcolor_2 (make `LinearColor` (`KismetMathLibrary.RandomFloatInRange` 0.3 1.0) (`KismetMathLibrary.RandomFloatInRange` 0.08 0.2) (`KismetMathLibrary.RandomFloatInRange` 0.02 0.1) 1.0))
  (bind _linearcolor_3 (make `LinearColor` (`KismetMathLibrary.RandomFloatInRange` 0.6 0.8) (`KismetMathLibrary.RandomFloatInRange` 0.1 0.4) (`KismetMathLibrary.RandomFloatInRange` 0.1 0.1) 1.0))
  (bind _linearcolor_4 (make `LinearColor` (`KismetMathLibrary.RandomFloatInRange` 0.0 1.0) (`KismetMathLibrary.RandomFloatInRange` 0.0 1.0) (`KismetMathLibrary.RandomFloatInRange` 0.02 1.0) 1.0))
  (bind _linearcolor_5 (make `LinearColor` (`KismetMathLibrary.RandomFloatInRange` 0.05 0.09) (`KismetMathLibrary.RandomFloatInRange` 0.04 0.09) (`KismetMathLibrary.RandomFloatInRange` 0.01 0.09) 1.0))
  (bind _linearcolor_6 (make `LinearColor` (`KismetMathLibrary.RandomFloatInRange` 0.6 1.0) (`KismetMathLibrary.RandomFloatInRange` 0.4 0.6) (`KismetMathLibrary.RandomFloatInRange` 0.1 0.2) 1.0))
  (bind _z (.z _boxextent))
  (bind _z_2 (.z (`SceneComponent.RelativeLocation` _body)))
  (bind _x (.x (`.BoxExtent` (`KismetSystemLibrary.GetComponentBounds` (`self.body`)))))
  (bind _returnvalue_2 (`KismetMathLibrary.MakeVector` 0.0 0.0 (.z (`SceneComponent.RelativeLocation` _body))))
  (bind _returnvalue_3 (- (.z (`SceneComponent.RelativeLocation` (`self.body`))) 70.0))
  (bind _returnvalue_4 (`KismetMathLibrary.MakeVector` (+ 0.0 (.x _boxextent_2)) 0.0 (- _z_2 (`self.handZLocation`))))
  (bind _returnvalue_5 (`KismetMathLibrary.MakeVector` (- 0.0 (.x _boxextent_2)) 0.0 (- _z_2 (`self.handZLocation`))))
  (bind _returnvalue_6 (`KismetMathLibrary.MakeVector` (- 0.0 _x) 0.0 _returnvalue_3))
  (bind _returnvalue_7 (`KismetMathLibrary.MakeVector` (+ 0.0 _x) 0.0 _returnvalue_3))
  (bind _returnvalue_8 (- (.x _returnvalue_5) (.x _boxextent)))
  (bind _returnvalue_9 (+ (.y _returnvalue_5) (* (.y _boxextent) 2.0)))
  (`|ExecutionSequence`
    (:`then_0`
      ;[1 1 1] скейл телу
      (`SceneComponent.SetRelativeScale3D` _body (`KismetMathLibrary.MakeVector` (`KismetMathLibrary.RandomFloatInRange` 3.0 8.0) (`KismetMathLibrary.RandomFloatInRange` 1.0 5.0) 7.0))
      (`SceneComponent.K2_SetRelativeTransform` (`self.head`) (`KismetMathLibrary.MakeTransform` _returnvalue_2 (struct) (2.5 2.5 2.5)) false false)
      (`SceneComponent.K2_SetRelativeLocation` (`self.PhysicsConstraint4`) _returnvalue_2 false false)
      (set `self.handScale` (`KismetMathLibrary.MakeVector` _returnvalue _returnvalue (`KismetMathLibrary.RandomFloatInRange` 4.0 8.0)))
      (set `self.legScale` (`KismetMathLibrary.MakeVector` (.x (`self.handScale`)) (.y (`self.handScale`)) 6.0))
      (set `self.handZLocation` (`KismetMathLibrary.RandomFloatInRange` 0.0 10.0))
      ;[1 1 1] трансформ правой руке
      (`SceneComponent.K2_SetRelativeTransform` _hand1 (`KismetMathLibrary.MakeTransform` _returnvalue_5 (`KismetMathLibrary.MakeRotator` (`KismetMathLibrary.RandomFloatInRange` -20.0 -90.0)) (`self.handScale`)) false false)
      (`SceneComponent.K2_SetRelativeTransform` (`self.PhysicsConstraint`) (`KismetMathLibrary.Conv_VectorToTransform` _returnvalue_5) false false)
      (`KismetSystemLibrary.PrintString` (`KismetStringLibrary.Conv_VectorToString` _boxextent) false false (struct :`G` 0.66 :`B` 1.0 :`A` 1.0) 8.0)
      (`SceneComponent.K2_SetRelativeTransform` _shovel (`KismetMathLibrary.MakeTransform` (`KismetMathLibrary.MakeVector` _returnvalue_8 _returnvalue_9 (- (.z _returnvalue_5) (+ _z (/ _z 2.0)))) (`KismetMathLibrary.MakeRotator` (`KismetMathLibrary.RandomFloatInRange` -10.0 10.0) (`KismetMathLibrary.RandomFloatInRange` -5.0 20.0)) (1.0 1.0 1.0)) false false)
      (`SceneComponent.K2_SetRelativeTransform` (`self.PhysicsConstraint5`) (`KismetMathLibrary.Conv_VectorToTransform` (`KismetMathLibrary.MakeVector` _returnvalue_8 _returnvalue_9 (- (.z (`SceneComponent.RelativeLocation` (`self.body`))) (.z (`.BoxExtent` (`KismetSystemLibrary.GetComponentBounds` _shovel)))))) false false)
      (`/Game/Blueprints/Utils.CreateDynamicMat` _shovel (struct :`R` 0.395 :`G` 0.343102 :`B` 0.25426 :`A` 1.0) (struct) 0 "/Game/Materials/simpleOneColor.simpleOneColor")
      (`/Game/Blueprints/Utils.CreateDynamicMatTextures` _shovel "/Game/Materials/simpleTexture.simpleTexture" (`self.boardTextures`) true 1.0 1.0 1)
      ;[1 1 1] трансформ левой руке
      (`SceneComponent.K2_SetRelativeTransform` (`self.hand2`) (`KismetMathLibrary.MakeTransform` _returnvalue_4 (struct) (`self.handScale`)) false false)
      (`SceneComponent.K2_SetRelativeTransform` (`self.PhysicsConstraint1`) (`KismetMathLibrary.Conv_VectorToTransform` _returnvalue_4) false false)
      ;[1 1 1] трансформ правой ноге
      (`SceneComponent.K2_SetRelativeTransform` (`self.leg1`) (`KismetMathLibrary.MakeTransform` _returnvalue_6 (struct) (`self.legScale`)) false false)
      (`SceneComponent.K2_SetRelativeTransform` (`self.PhysicsConstraint2`) (`KismetMathLibrary.Conv_VectorToTransform` _returnvalue_6) false false)
      ;[1 1 1] трансформ левой ноге
      (`SceneComponent.K2_SetRelativeTransform` (`self.leg2`) (`KismetMathLibrary.MakeTransform` _returnvalue_7 (struct) (`self.legScale`)) false false)
      (`SceneComponent.K2_SetRelativeTransform` (`self.PhysicsConstraint3`) (`KismetMathLibrary.Conv_VectorToTransform` _returnvalue_7) false false))
    (:`then_1`
      (`self.GenerateColors`)
      (set `self.sleeveLength` (`KismetMathLibrary.RandomFloatInRange` 0.5 1.0))
      (set `self.pantsLength` (`KismetMathLibrary.RandomFloatInRange` 0.6 1.0))
      (set `self.eyesScale` (`KismetMathLibrary.MakeVector` (`KismetMathLibrary.RandomFloatInRange` 0.01 0.04) 0.01 (`KismetMathLibrary.RandomFloatInRange` 0.01 0.04)))
      (`/Game/Blueprints/Utils.CreateDynamicMat` _eye1 _eyescolor (struct) 0 "/Game/Materials/simpleOneColor.simpleOneColor")
      (`/Game/Blueprints/Utils.CreateDynamicMat` _eye2 _eyescolor (struct) 0 "/Game/Materials/simpleOneColor.simpleOneColor")
      (`SceneComponent.SetRelativeScale3D` _eye1 (`self.eyesScale`))
      (`SceneComponent.SetRelativeScale3D` _eye2 (`self.eyesScale`))
      (`SceneComponent.SetRelativeScale3D` _mouth (`KismetMathLibrary.MakeVector` (`KismetMathLibrary.RandomFloatInRange` 0.01 0.1) 0.01 (`KismetMathLibrary.RandomFloatInRange` 0.01 0.02)))
      (`/Game/Blueprints/Utils.CreateDynamicMat` _mouth (make `LinearColor` (`KismetMathLibrary.RandomFloatInRange` 0.1 0.3) (`KismetMathLibrary.RandomFloatInRange` 0.0 0.1) (`KismetMathLibrary.RandomFloatInRange` 0.0 0.1) 1.0) (struct) 0 "/Game/Materials/simpleOneColor.simpleOneColor")
      (`|ExecutionSequence`
        (:`then_0`
          (set `self.randomHairColor` (`KismetMathLibrary.RandomIntegerInRange` 0 19))
          ;[1 1 1] темные волосы
          (if (> (`self.randomHairColor`) 12)
            (`/Game/Blueprints/Utils.CreateDynamicMat` (`self.head`) _linearcolor_5 (make `LinearColor` (`KismetMathLibrary.RandomFloatInRange` 0.05 0.09) (`KismetMathLibrary.RandomFloatInRange` 0.04 0.09) (`KismetMathLibrary.RandomFloatInRange` 0.01 0.09) 1.0) 1 "/Game/Materials/simple2colorGradHorizontal.simple2colorGradHorizontal")
            (set `self.hairColor` _linearcolor_5)
            (else
              ;[1 1 1] светлые волосы
              (if (> (`self.randomHairColor`) 4)
                (`/Game/Blueprints/Utils.CreateDynamicMat` (`self.head`) _linearcolor_6 (make `LinearColor` (`KismetMathLibrary.RandomFloatInRange` 0.6 1.0) (`KismetMathLibrary.RandomFloatInRange` 0.4 0.6) (`KismetMathLibrary.RandomFloatInRange` 0.1 0.2) 1.0) 1 "/Game/Materials/simple2colorGradHorizontal.simple2colorGradHorizontal")
                (set `self.hairColor` _linearcolor_6)
                (else
                  ;[1 1 1] рыжие волосы
                  (if (>= (`self.randomHairColor`) 1)
                    (`/Game/Blueprints/Utils.CreateDynamicMat` (`self.head`) _linearcolor_2 (make `LinearColor` (`KismetMathLibrary.RandomFloatInRange` 0.3 1.0) (`KismetMathLibrary.RandomFloatInRange` 0.08 0.2) (`KismetMathLibrary.RandomFloatInRange` 0.01 0.1) 1.0) 1 "/Game/Materials/simple2colorGradHorizontal.simple2colorGradHorizontal")
                    (set `self.hairColor` _linearcolor_2)
                    (else
                      ;[1 1 1] цветные волосы
                      (if (== (`self.randomHairColor`) 0)
                        (`/Game/Blueprints/Utils.CreateDynamicMat` (`self.head`) _linearcolor_4 (make `LinearColor` (`KismetMathLibrary.RandomFloatInRange` 0.0 1.0) (`KismetMathLibrary.RandomFloatInRange` 0.0 1.0) (`KismetMathLibrary.RandomFloatInRange` 0.0 1.0) 1.0) 1 "/Game/Materials/simple2colorGradHorizontal.simple2colorGradHorizontal")
                        (set `self.hairColor` _linearcolor_4)))))))))
        (:`then_1`
          ;[1 1 1] цвет лица
          (if (== (`KismetMathLibrary.RandomIntegerInRange` 0 12) 0)
            (bind _dynamicmaterial (`/Game/Blueprints/Utils.CreateDynamicMat` (`self.head`) _linearcolor (`self.hairColor`) 0 "/Game/Materials/simple2colorGradSharpen.simple2colorGradSharpen"))
            (`MaterialInstanceDynamic.SetScalarParameterValue` _dynamicmaterial "vertTiles" (`KismetMathLibrary.RandomFloatInRange` 0.0 1.0))
            (set `self.skinColor` _linearcolor)
            (else
              (bind _dynamicmaterial_2 (`/Game/Blueprints/Utils.CreateDynamicMat` (`self.head`) _linearcolor_3 (`self.hairColor`) 0 "/Game/Materials/simple2colorGradSharpen.simple2colorGradSharpen"))
              (`MaterialInstanceDynamic.SetScalarParameterValue` _dynamicmaterial_2 "vertTiles" (`KismetMathLibrary.RandomFloatInRange` 0.0 0.8))
              (set `self.skinColor` _linearcolor_3))))
        (:`then_2`
          ;[1 1 1] цвет и длина рукавов и рук
          (bind _dynamicmaterial_3 (`/Game/Blueprints/Utils.CreateDynamicMat` (`self.hand1`) (`self.coatColor`) (`self.skinColor`) 0 "/Game/Materials/simple2colorGradSharpen.simple2colorGradSharpen"))
          (`MaterialInstanceDynamic.SetScalarParameterValue` _dynamicmaterial_3 "vertTiles" (`self.sleeveLength`))
          (bind _dynamicmaterial_4 (`/Game/Blueprints/Utils.CreateDynamicMat` (`self.hand2`) (`self.coatColor`) (`self.skinColor`) 0 "/Game/Materials/simple2colorGradSharpen.simple2colorGradSharpen"))
          (`MaterialInstanceDynamic.SetScalarParameterValue` _dynamicmaterial_4 "vertTiles" (`self.sleeveLength`))
          ;[1 1 1] цвет и длина штанов
          (bind _dynamicmaterial_5 (`/Game/Blueprints/Utils.CreateDynamicMat` (`self.leg1`) (`self.pantsColor`) (`self.shoesColor`) 0 "/Game/Materials/simple2colorGradSharpen.simple2colorGradSharpen"))
          (`MaterialInstanceDynamic.SetScalarParameterValue` _dynamicmaterial_5 "vertTiles" (`self.pantsLength`))
          (bind _dynamicmaterial_6 (`/Game/Blueprints/Utils.CreateDynamicMat` (`self.leg2`) (`self.pantsColor`) (`self.shoesColor`) 0 "/Game/Materials/simple2colorGradSharpen.simple2colorGradSharpen"))
          (`MaterialInstanceDynamic.SetScalarParameterValue` _dynamicmaterial_6 "vertTiles" (`self.pantsLength`))
          (if (== (`KismetMathLibrary.RandomIntegerInRange` 0 1) 0)
            ;[1 1 1] цвет и длина курточки
            (bind _dynamicmaterial_7 (`/Game/Blueprints/Utils.CreateDynamicMat` (`self.body`) (`self.coatColor`) (`self.pantsColor`) 0 "/Game/Materials/simple2colorGradSharpenMirrorV.simple2colorGradSharpenMirrorV"))
            (`MaterialInstanceDynamic.SetScalarParameterValue` _dynamicmaterial_7 "vertTiles" (`KismetMathLibrary.RandomFloatInRange` 0.2 1.0))
            (else
              ;[1 1 1] цвет и длина курточки и юбки
              (bind _dynamicmaterial_8 (`/Game/Blueprints/Utils.CreateDynamicMat` (`self.body`) (`self.coatColor`) (make `LinearColor` (`KismetMathLibrary.RandomFloatInRange` 0.01 1.0) (`KismetMathLibrary.RandomFloatInRange` 0.01 1.0) (`KismetMathLibrary.RandomFloatInRange` 0.01 1.0) 1.0) 0 "/Game/Materials/simple2colorGradSharpenMirrorV.simple2colorGradSharpenMirrorV"))
              (`MaterialInstanceDynamic.SetScalarParameterValue` _dynamicmaterial_8 "vertTiles" (`KismetMathLibrary.RandomFloatInRange` 0.2 1.0)))))))))
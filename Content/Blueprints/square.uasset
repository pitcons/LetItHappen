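; Square tile actor Blueprint that randomizes the look and height of its static mesh pieces in the Construction Script.
; It loops over the root's child meshes, setting each to a custom collision object channel and calling CreateDynamicMat with SquareTiles and a slightly randomized dark color.
; Every mesh not named "platform" gets a random relative Z offset, creating an uneven surface, and each mesh name is printed for debugging.
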(fn `UserConstructionScript`
  (for _array_element (`SceneComponent.GetChildrenComponents` (`self.DefaultSceneRoot`) false)
    (bind _asstatic_mesh_component (cast `StaticMeshComponent` _array_element))
    (`PrimitiveComponent.SetCollisionObjectType` _asstatic_mesh_component "ECC_GameTraceChannel1")
    (`/Game/Blueprints/Utils.CreateDynamicMat` _asstatic_mesh_component (make `LinearColor` (`KismetMathLibrary.RandomFloatInRange` 0.025 0.035) (`KismetMathLibrary.RandomFloatInRange` 0.025 0.035) (`KismetMathLibrary.RandomFloatInRange` 0.025 0.035) 1.0) (struct :`A` 1.0) 0 "/Game/Materials/squareTiles.squareTiles")
    (bind _returnvalue (`KismetSystemLibrary.GetObjectName` _asstatic_mesh_component))
    (`KismetSystemLibrary.PrintString` _returnvalue false false)
    (if (`KismetStringLibrary.NotEqual_StrStr` _returnvalue "platform")
      (`SceneComponent.K2_SetRelativeLocation` _asstatic_mesh_component (`KismetMathLibrary.MakeVector` (.x (`SceneComponent.RelativeLocation` _asstatic_mesh_component)) (.y (`SceneComponent.RelativeLocation` _asstatic_mesh_component)) (`KismetMathLibrary.RandomFloatInRange` 0.0 50.0)) false false))))
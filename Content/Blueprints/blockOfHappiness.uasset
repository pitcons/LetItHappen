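; An actor with a Cube component that periodically switches physics simulation on and off.
; Tick accumulates delta time in TickDelay, enabling physics on the cube once it passes eleven seconds.
; At thirteen seconds it disables physics and resets the timer, so the cube simulates for about two seconds per cycle.
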(event `self.ReceiveTick`
  (params (DeltaSeconds :type "Float (single-precision)"))
  (set `self.tickDelay` (+ DeltaSeconds (`self.tickDelay`)))
  (if (>= (`self.tickDelay`) 11.0)
    (`PrimitiveComponent.SetSimulatePhysics` (`self.Cube`) true))
  (if (>= (`self.tickDelay`) 13.0)
    (`PrimitiveComponent.SetSimulatePhysics` (`self.Cube`) false)
    (set `self.tickDelay` 0.0)))

(fn `UserConstructionScript`)
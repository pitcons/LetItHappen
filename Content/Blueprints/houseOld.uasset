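; houseOld is a house actor that randomizes its size and wall colors in the construction script.
; It scales the static mesh by random whole-number width and height, leaving depth fixed.
; CreateDynamicMat applies HouseWallWindows with two random colors, one darker, and UV values proportional to that scale, so the window pattern follows building size.
; The event graph has no active logic.
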(fn `UserConstructionScript`
  (set `self.U` (`KismetMathLibrary.Conv_IntToDouble` (`KismetMathLibrary.RandomIntegerInRange` 1 3)))
  (set `self.V` (`KismetMathLibrary.Conv_IntToDouble` (`KismetMathLibrary.RandomIntegerInRange` 1 3)))
  (`SceneComponent.SetRelativeScale3D` (`self.StaticMeshComponent`) (`KismetMathLibrary.MakeVector` (`self.U`) (`KismetMathLibrary.Conv_IntToDouble` (`KismetMathLibrary.RandomIntegerInRange` 1 1)) (`self.V`)))
  (`/Game/Blueprints/Utils.CreateDynamicMat` (`self.StaticMeshComponent`) (make `LinearColor` (`KismetMathLibrary.RandomFloatInRange` 0.1 0.4) (`KismetMathLibrary.RandomFloatInRange` 0.1 0.4) (`KismetMathLibrary.RandomFloatInRange` 0.1 0.4) 1.0) (make `LinearColor` (`KismetMathLibrary.RandomFloatInRange` 0.01 0.15) (`KismetMathLibrary.RandomFloatInRange` 0.01 0.15) (`KismetMathLibrary.RandomFloatInRange` 0.01 0.15) 1.0) 0 "/Game/Materials/houseWallWindows.houseWallWindows" true (* (`self.U`) 3.0) (* (`self.V`) 3.0)))
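; houseModern is a procedural modern building actor that randomizes its shape and wall look in the construction script.
; It scales its static mesh to a random whole-number footprint and height, mostly tall.
; CreateDynamicMat builds a dynamic HouseModernWall material with random dark colors and UV tiling derived from that scale.
; Extra random scalar and color parameters add further variety, while the event graph stays unused.
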(fn `UserConstructionScript`
  (set `self.U` (`KismetMathLibrary.Conv_IntToDouble` (`KismetMathLibrary.RandomIntegerInRange` 1 3)))
  (set `self.V` (`KismetMathLibrary.Conv_IntToDouble` (`KismetMathLibrary.RandomIntegerInRange` 4 15)))
  (`SceneComponent.SetRelativeScale3D` (`self.StaticMeshComponent`) (`KismetMathLibrary.MakeVector` (`self.U`) (`KismetMathLibrary.Conv_IntToDouble` (`KismetMathLibrary.RandomIntegerInRange` 1 2)) (`self.V`)))
  (bind _dynamicmaterial (`/Game/Blueprints/Utils.CreateDynamicMat` (`self.StaticMeshComponent`) (make `LinearColor` (`KismetMathLibrary.RandomFloatInRange` 0.01 0.4) (`KismetMathLibrary.RandomFloatInRange` 0.01 0.4) (`KismetMathLibrary.RandomFloatInRange` 0.01 0.4) 1.0) (make `LinearColor` (`KismetMathLibrary.RandomFloatInRange` 0.01 0.4) (`KismetMathLibrary.RandomFloatInRange` 0.01 0.4) (`KismetMathLibrary.RandomFloatInRange` 0.01 0.4) 1.0) 0 "/Game/Materials/houseModernWall.houseModernWall" true (* (`self.U`) (`KismetMathLibrary.Conv_IntToDouble` (`KismetMathLibrary.RandomIntegerInRange` 1 20))) (* (`self.V`) (`KismetMathLibrary.Conv_IntToDouble` (`KismetMathLibrary.RandomIntegerInRange` 2 4)))))
  (`MaterialInstanceDynamic.SetScalarParameterValue` _dynamicmaterial "U1" (`KismetMathLibrary.Conv_IntToDouble` (`KismetMathLibrary.RandomIntegerInRange` 0 10)))
  (`MaterialInstanceDynamic.SetVectorParameterValue` _dynamicmaterial "extraColor1" (make `LinearColor` (`KismetMathLibrary.RandomFloatInRange` 0.01 0.7) (`KismetMathLibrary.RandomFloatInRange` 0.01 0.7) (`KismetMathLibrary.RandomFloatInRange` 0.01 0.7) 1.0))
  (`MaterialInstanceDynamic.SetVectorParameterValue` _dynamicmaterial "extraColor2" (make `LinearColor` (`KismetMathLibrary.RandomFloatInRange` 0.01 0.7) (`KismetMathLibrary.RandomFloatInRange` 0.01 0.7) (`KismetMathLibrary.RandomFloatInRange` 0.01 0.7) 1.0)))
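; AgroCheck is a behavior tree node that looks for visible targets around a Follower_AI_CON-controlled pawn on each tick.
; It caches the controller, then sphere-traces nearby objects of the desired types, ignoring all AI_Character actors.
; Each hit gets a Camera-channel line-of-sight trace: visible ones set TargetToFollow and TargetLocation, blocked ones clear TargetToFollow, so later hits override earlier ones.
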(event `self.ReceiveTick`
  (params (OwnerActor :type "Actor Object Reference") (DeltaSeconds :type "Float (single-precision)"))
  (bind _returnvalue (`Actor.K2_GetActorLocation` (`Controller.K2_GetPawn` (`self.AI_CON_Ref`))))
  ;[1 1 1] Is AI CON ref set?
  (if (!= (`self.AI_CON_Ref`) null)
    (`KismetSystemLibrary.PrintString` "we")
    (else
      (bind _asfollower_ai_con (cast `/Game/Blueprints/AI/Follower_AI_CON` OwnerActor))
      (set `self.AI_CON_Ref` _asfollower_ai_con)))
  (bind _outactors (`GameplayStatics.GetAllActorsOfClass` "/Game/Blueprints/AI/AI_Character.AI_Character_C"))
  (set `self.MyLocation` _returnvalue)
  (bind _outhits (`KismetSystemLibrary.SphereTraceMultiForObjects` _returnvalue (+ _returnvalue (0.0 0.0 15.0)) 1500.0 (`self.DesiredObjectTypes`) false _outactors))
  (for _array_element _outhits
    (bind (_bblockinghit _binitialoverlap _time _location _impactpoint _normal _impactnormal _physmat _hitactor) (`GameplayStatics.BreakHitResult` _array_element))
    (bind _outhit (`KismetSystemLibrary.LineTraceSingle` (`self.MyLocation`) (`Actor.K2_GetActorLocation` _hitactor) "TraceTypeQuery2" false _outactors))
    (bind (_bblockinghit_2 _binitialoverlap_2 _time_2 _location_2 _impactpoint_2 _normal_2 _impactnormal_2 _physmat_2 _hitactor_2) (`GameplayStatics.BreakHitResult` _outhit))
    (if (== _hitactor_2 _hitactor)
      (`BTFunctionLibrary.SetBlackboardValueAsObject` (`self.TargetToFollow`) _hitactor_2)
      (bind _returnvalue_2 (`Actor.K2_GetActorLocation` _hitactor_2))
      (`BTFunctionLibrary.SetBlackboardValueAsVector` (`self.TargetLocation`) _returnvalue_2)
      (`KismetSystemLibrary.PrintString` (`KismetStringLibrary.Concat_StrStr` "new TargetLocation" (`KismetStringLibrary.Conv_VectorToString` _returnvalue_2)))
      (else
        (`BTFunctionLibrary.SetBlackboardValueAsObject` (`self.TargetToFollow`))))))
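; RapidMoveTo is a behavior tree task that moves the pawn of a Follower_AI_CON controller.
; On execute it caches the controller, then calls AIMoveTo with the TargetToFollow blackboard actor as target and a hardcoded world location as destination.
; It finishes successfully when the move succeeds, with debug prints along the way.
; Move failure and a failed controller cast never call FinishExecute.
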(event `self.ReceiveExecute`
  (params (OwnerActor :type "Actor Object Reference"))
  (if (not (!= (`self.AI_CON_Ref`) null))
    (bind _asfollower_ai_con (cast `/Game/Blueprints/AI/Follower_AI_CON` OwnerActor))
    (set `self.AI_CON_Ref` _asfollower_ai_con))
  (`KismetSystemLibrary.PrintString` "Run backward")
  (`|AIMoveTo` (`Controller.K2_GetPawn` (`self.AI_CON_Ref`)) (-1521.0 2260.0 96.0) (`BTFunctionLibrary.GetBlackboardValueAsActor` (`self.TargetToFollow`)) 50.0
    (:`OnSuccess`
      (`self.FinishExecute` true)
      (`KismetSystemLibrary.PrintString` "Rapid Move To Finish"))))